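; Finn, the PaperZD side-scroller player character, with Enhanced Input movement, jumping, death and respawn at the starting location.
; Coyote time permits jumps shortly after leaving a ledge, and control rotation follows horizontal velocity.
; Each tick drives delayed spring-arm look-ahead and a vertical deadzone camera that follows Z through timelines outside jump bounds.
; Damage freezes movement and plays death animation, falling too low or pressing R respawns, and KillBox overlaps damage interface actors.
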(event `self.ReceiveBeginPlay`
  (bind (_returnvalue_x _returnvalue_y _returnvalue_z) (`KismetMathLibrary.BreakVector` (`self.K2_GetActorLocation`)))
  (`|ExecutionSequence`
    (:`then_0`
      (bind _asplayer_controller (cast `PlayerController` (`self.GetController`)))
      (`EnhancedInputSubsystemInterface.AddMappingContext` (pcsubsystem `EnhancedInputLocalPlayerSubsystem` _asplayer_controller) "/Game/2dSandbox/SideScroller/Input/IMC_SideScroller.IMC_SideScroller" 0 (struct)))
    (:`then_1`
      (set `CharacterMovementComponent.JumpZVelocity` (`self.Intial Jump Velocity`) (`self.CharacterMovement`))
      (set `self.JumpMaxHoldTime` (`self.Jump Max Hold Time`)))
    (:`then_2`
      ;[1 1 1] Respawn location
      (set `self.Respawn Location` (`self.K2_GetActorLocation`)))
    (:`then_3`
      (add `self.OnDestroyed` (delegate `OnDestroyed_Event`)))
    (:`then_4`
      (set `self.LastZLocation` _returnvalue_z))))

(event `OnDestroyed_Event` :!signature `self.OnDestroyed`
  (params (DestroyedActor :type "Actor Object Reference"))
  (`self.Take Fall Damage`))

(event `self.ReceiveTick`
  (params (DeltaSeconds :type "Float (single-precision)"))
  (`self.Update Control Rotation`)
  (`self.LookAhead` false)
  (`self.SetJumpTarget`)
  (`self.CheckFallDamage`))

(event `self.K2_OnMovementModeChanged`
  (params (PrevMovementMode :type "EMovementMode Enum" :default "MOVE_None") (NewMovementMode :type "EMovementMode Enum" :default "MOVE_None") (PrevCustomMode :type Byte) (NewCustomMode :type Byte))
  (if (and (`|EnumEquality` PrevMovementMode "MOVE_Walking") (`|EnumEquality` NewMovementMode "MOVE_Falling") (not (`self.IsJumping`)))
    (`self.Start CoyoteTime Timer`)))

(event `Start CoyoteTime Timer`
  (set `self.IsCoyoteTimeActive?` true)
  (`KismetSystemLibrary.K2_SetTimerDelegate` (delegate `CoyoteTimerFinished`) 0.2))

(event `CoyoteTimerFinished`
  (set `self.IsCoyoteTimeActive?` false))

(event `self.OnLanded`
  (params (Hit :type "HitResult Structure (by ref)"))
  (set `self.IsJumping` false))

(event `self.ReceiveAnyDamage`
  (params (Damage :type "Float (single-precision)") (DamageType :type "DamageType Object Reference") (InstigatedBy :type "Controller Object Reference") (DamageCauser :type "Actor Object Reference"))
  ;[1 1 1] Player Death
  (set `self.IsDead` true :!label _label)
  (`PaperZDAnimInstance.JumpToNode` (`PaperZDAnimationComponent.AnimInstance` (`self.AnimationComponent`)) "PlayerDead" "None")
  (`ActorComponent.SetActive` (`self.CharacterMovement`) false false))

(event `/Game/Blueprints/DamageAbleBPI.TakeDamage`
  (goto _label))

(event `Take Fall Damage`
  (`self.Respawn player character`))

(event `Respawn player character`
  (bind (_returnvalue_x _returnvalue_y _returnvalue_z) (`KismetMathLibrary.BreakVector` (`self.K2_GetActorLocation`)))
  ;[1 1 1] Respawn
  (`self.K2_SetActorLocation` (`self.Respawn Location`))
  (set `self.IsDead` false)
  (`ActorComponent.SetActive` (`self.CharacterMovement`) true false)
  (set `self.LastZLocation` _returnvalue_z))

(event `Key|R`
  (params (Key :type "Key Structure"))
  (:`Pressed`
    (`self.Respawn player character`)))

(event `CheckFallDamage`
  (if (<= (.z (`self.K2_GetActorLocation`)) -800.0)
    (`self.Respawn player character`)))

(event `EnhancedInput|/Game/2dSandbox/SideScroller/Input/Input_Actions/IA_2D_Jump`
  (params (ActionValue :type Boolean) (ElapsedSeconds :type "Float (double-precision)") (TriggeredSeconds :type "Float (double-precision)") (InputAction :type "InputAction Object Reference" :default "/Game/2dSandbox/SideScroller/Input/Input_Actions/IA_2D_Jump.IA_2D_Jump"))
  (:`Triggered`
    (if (`self.IsCoyoteTimeActive?`)
      (`CharacterMovementComponent.SetMovementMode` (`self.CharacterMovement`) "MOVE_Walking" 0))
    (`self.Jump`)
    (set `self.IsJumping` true)
    (set `self.IsCoyoteTimeActive?` false))
  (:`Canceled`
    (`self.StopJumping` :!label _label))
  (:`Completed`
    (goto _label)))

(event `self.OnWalkingOffLedge`
  (params (PreviousFloorImpactNormal :type "Vector Structure (by ref)") (PreviousFloorContactNormal :type "Vector Structure (by ref)") (PreviousLocation :type "Vector Structure (by ref)") (TimeDelta :type "Float (single-precision)"))
  (`PaperZDAnimInstance.JumpToNode` (`PaperZDAnimationComponent.AnimInstance` (`self.AnimationComponent`)) "Airborne" "None" :!label _label_2))

(event `EnhancedInput|/Game/2dSandbox/SideScroller/Input/Input_Actions/IA_2D_Move`
  (params (ActionValue :type "Float (double-precision)") (ElapsedSeconds :type "Float (double-precision)") (TriggeredSeconds :type "Float (double-precision)") (InputAction :type "InputAction Object Reference" :default "/Game/2dSandbox/SideScroller/Input/Input_Actions/IA_2D_Move.IA_2D_Move"))
  (bind _returnvalue (`self.GetVelocity`))
  (:`Triggered`
    (`self.AddMovementInput` (1.0 0.0 0.0) ActionValue)
    (bind (_direction _zvalue) (`Timeline|Timeline_0`)
      (:`Update`
        (set `MovementComponent.Velocity` (`KismetMathLibrary.VLerp` _returnvalue (`KismetMathLibrary.Vector_ClampSizeMax` _returnvalue 400.0) _zvalue) (`self.CharacterMovement`))
        (`KismetSystemLibrary.PrintString` (`KismetStringLibrary.Conv_DoubleToString` (`KismetMathLibrary.VSize` (`self.GetVelocity`))) true false (struct :`G` 0.66 :`B` 1.0 :`A` 1.0) 1.0 "-1")))))

(event `self.OnJumped`
  (goto _label_2))

(event `Update Animation`
  ;[1 1 1] Player Death animation
  (if (not (`self.IsDead`))
    (`PaperFlipbookComponent.SetFlipbook` (`self.Sprite`) (select `bool` (`NavMovementComponent.IsFalling` (`self.CharacterMovement`)) :`false` (select `bool` (> (`KismetMathLibrary.VSize` (`MovementComponent.Velocity` (`self.CharacterMovement`))) 0.0) :`false` (`self.Idle Animation`) :`true` (`self.Run Animation`)) :`true` (`self.Fall Animation`)))))

(event `Update Control Rotation`
  (`/Engine/EditorBlueprintResources/StandardMacros.IsValid` (`self.GetController`)
    (:`Is Valid`
      (`/Engine/EditorBlueprintResources/StandardMacros.CompareFloat` (.x (`MovementComponent.Velocity` (`self.CharacterMovement`)))
        (:`>`
          (`Controller.SetControlRotation` (`self.GetController`) (`KismetMathLibrary.MakeRotator` 0.0))
          (set `self.Direction` 1.0))
        (:`==`
          (set `self.Direction` 0.0))
        (:`<`
          (`Controller.SetControlRotation` (`self.GetController`) (`KismetMathLibrary.MakeRotator` 0.0 0.0 180.0))
          (set `self.Direction` -1.0))))))

(event `ResetLookAhead`
  (bind _targetoffset_x (`KismetMathLibrary.BreakVector` (`SpringArmComponent.TargetOffset` (`self.SpringArm`))))
  (if (!= (`self.Direction`) 0.0) :!label _label
    (set `SpringArmComponent.TargetOffset` (`KismetMathLibrary.MakeVector` (`KismetMathLibrary.Lerp` _targetoffset_x (* (`self.Look Ahead Distance`) (`self.Direction`)) 0.5)) (`self.SpringArm`))))

(event `LookAhead`
  (params (`Forward?` :type Boolean))
  (`KismetSystemLibrary.Delay` 1.0)
  (`|ExecutionSequence`
    (:`then_0`
      (goto _label))
    (:`then_1`
      (`self.ZoomOut`))))

(event `ZoomOut`)

(event `SetJumpTarget`
  (bind (_returnvalue_x _returnvalue_y _returnvalue_z) (`KismetMathLibrary.BreakVector` (`self.K2_GetActorLocation`)))
  (bind (_returnvalue_x_2 _returnvalue_y_2) (`KismetMathLibrary.BreakVector` (`self.K2_GetActorLocation`)))
  (bind (_returnvalue_x_3 _returnvalue_y_3 _returnvalue_z_2) (`KismetMathLibrary.BreakVector` (`self.K2_GetActorLocation`)))
  (bind (_returnvalue_x_4 _returnvalue_y_4 _returnvalue_z_3) (`KismetMathLibrary.BreakVector` (`self.K2_GetActorLocation`)))
  (bind (_returnvalue_x_5 _returnvalue_y_5) (`KismetMathLibrary.BreakVector` (`self.K2_GetActorLocation`)))
  (bind (_returnvalue_x_6 _returnvalue_y_6 _returnvalue_z_4) (`KismetMathLibrary.BreakVector` (`SceneComponent.K2_GetComponentLocation` (`self.SpringArm`))))
  (bind (_returnvalue_x_7 _returnvalue_y_7 _returnvalue_z_5) (`KismetMathLibrary.BreakVector` (`SceneComponent.K2_GetComponentLocation` (`self.SpringArm`))))
  (bind (_targetoffset_x _targetoffset_y _targetoffset_z) (`KismetMathLibrary.BreakVector` (`SpringArmComponent.TargetOffset` (`self.SpringArm`))))
  (bind (_isinbounds_ _upper_bounds _lowerbounds) (`self.CalculateJumpBounds` _returnvalue_z (`self.Max Height`) (`self.Min Height`) _targetoffset_z))
  (set `self.Upper Bounds` _upper_bounds)
  (set `self.Lower Bounds` _lowerbounds)
  (set `self.Is in Bounds?` _isinbounds_)
  (`self.DrawBounds` (`self.Upper Bounds`) (`self.ShowDebugInfo`))
  (`self.DrawBounds` (`self.Lower Bounds`) (`self.ShowDebugInfo`))
  (if _isinbounds_
    (bind (_direction _zvalue) (`Timeline|Timeline`)
      (:`Update`
        (`SceneComponent.K2_SetWorldLocation` (`self.SpringArm`) (`KismetMathLibrary.MakeVector` _returnvalue_x_2 _returnvalue_y_2 (`KismetMathLibrary.Lerp` _returnvalue_z_4 (`self.LastZLocation`) _zvalue)) false false)))
    (else
      (set `self.LastZLocation` _returnvalue_z_3)
      (bind (_direction_2 _zvalue_2) (`Timeline|MoveTOposition`)
        (:`Update`
          (`SceneComponent.K2_SetWorldLocation` (`self.SpringArm`) (`KismetMathLibrary.MakeVector` _returnvalue_x_5 _returnvalue_y_5 (`KismetMathLibrary.Lerp` _returnvalue_z_5 (`self.LastZLocation`) _zvalue_2)) false false))
        (:`Finished`
          (set `self.LastZLocation` _returnvalue_z_2))))))

(event `self.KillBox.OnComponentBeginOverlap`
  (params (OverlappedComponent :type "PrimitiveComponent Object Reference") (OtherActor :type "Actor Object Reference") (OtherComp :type "PrimitiveComponent Object Reference") (OtherBodyIndex :type Integer) (bFromSweep :type Boolean) (SweepResult :type "HitResult Structure (by ref)"))
  (if (`KismetSystemLibrary.DoesImplementInterface` OtherActor "/Game/Blueprints/DamageAbleBPI.DamageAbleBPI_C")
    (message `/Game/Blueprints/DamageAbleBPI.TakeDamage` OtherActor)))

(fn `UserConstructionScript`)